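; Bomb countdown actor that quits the game when its timer runs out.
; Tick checks the FromSweep output of the otherwise unwired BombTriggerArea begin-overlap event to decide whether to count down.
; A one-second Delay inside Tick paces the loop, decrementing the Integer counter and writing it to the Countdown text.
; Once the counter drops to -1 or below, the game quits.
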(event `self.ReceiveTick`
  (params (DeltaSeconds :type "Float (single-precision)"))
  (if (stale `self.Bomb Trigger Area.OnComponentBeginOverlap` bFromSweep)
    (`KismetSystemLibrary.Delay` 1.0)
    (set `self.Integer` (- (`self.Integer`) 1))
    (`TextRenderComponent.K2_SetText` (`self.Countdown`) (`KismetTextLibrary.Conv_IntToText` (`self.Integer`)))
    ;[1 1 1] If Integer is <or= -1 Game will end run out of time
    (if (<= (`self.Integer`) -1)
      (`KismetSystemLibrary.QuitGame` null "Quit"))))

(event `self.Bomb Trigger Area.OnComponentBeginOverlap`
  (params (OverlappedComponent :type "PrimitiveComponent Object Reference") (OtherActor :type "Actor Object Reference") (OtherComp :type "PrimitiveComponent Object Reference") (OtherBodyIndex :type Integer) (bFromSweep :type Boolean) (SweepResult :type "HitResult Structure (by ref)")))

(fn `UserConstructionScript`)